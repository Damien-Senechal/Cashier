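; BP_CashRegister is a cash register that detects BP_Items with a scanner and pushes them along.
; Each tick it runs a visibility box trace above the Scanner's relative location, drawing debug and printing the hit component's name.
; When the hit component is the item's Box, it calls DesactivateScanPhase on the item and overrides its mesh's physics velocity toward negative Y.
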(event `self.ReceiveTick`
  (params (DeltaSeconds :type "Float (single-precision)"))
  (bind _scanner (`self.Scanner`))
  (bind (_relativelocation_x _relativelocation_y _relativelocation_z) (`KismetMathLibrary.BreakVector` (`SceneComponent.RelativeLocation` _scanner)))
  (bind (_relativelocation_x_2 _relativelocation_y_2 _relativelocation_z_2) (`KismetMathLibrary.BreakVector` (`SceneComponent.RelativeLocation` _scanner)))
  (bind _outhit (`KismetSystemLibrary.BoxTraceSingle` :`Start` (`KismetMathLibrary.MakeVector` _relativelocation_x_2 _relativelocation_y_2 (+ _relativelocation_z_2 300.0)) :`End` (`KismetMathLibrary.MakeVector` _relativelocation_x _relativelocation_y (+ _relativelocation_z 400.0)) :`HalfSize` (50.0 75.0 0.0) :`TraceChannel` "TraceTypeQuery1" :`DrawDebugType` "ForOneFrame"))
  (`KismetSystemLibrary.PrintString` (`KismetSystemLibrary.GetDisplayName` (`.HitComponent` (`GameplayStatics.BreakHitResult` _outhit))))
  (bind _asbp_items (cast `/Game/BP/Items/BP_Items` (`.HitActor` (`GameplayStatics.BreakHitResult` _outhit))))
  (if (== (`.HitComponent` (`GameplayStatics.BreakHitResult` _outhit)) (`/Game/BP/Items/BP_Items.Box` _asbp_items))
    (`/Game/BP/Items/BP_Items.DesactivateScanPhase` _asbp_items)
    (`PrimitiveComponent.SetAllPhysicsLinearVelocity` (`/Game/BP/Items/BP_Items.StaticMesh` _asbp_items) (0.0 -500.0 0.0) false)))

(fn `UserConstructionScript`)