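; BP_Items is a physics item that the player clicks to place at the cash register's inspection point and rotate with the mouse for scanning.
; Clicking triggers ActivateScanPhase, which gets the register through the game mode, moves the mesh, disables physics, hides the cursor and enables input.
; Mouse axes rotate the actor while inspecting.
; DesactivateScanPhase, not called within this Blueprint, restores physics and cursor and disables input.
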(event `self.StaticMesh.OnClicked`
  (params (TouchedComponent :type "PrimitiveComponent Object Reference") (ButtonPressed :type "Key Structure"))
  (if (and (`self.IsOnScanner`) (`self.IsRotating`))
    (`KismetSystemLibrary.PrintString` "Deja sur le scanner")
    (else
      (`self.ActivateScanPhase`))))

(event `InputAxisKey|MouseX`
  (params (AxisValue :type "Float (single-precision)"))
  (if (`self.IsRotating`)
    (`self.K2_SetActorRotation` (`KismetMathLibrary.ComposeRotators` (`self.K2_GetActorRotation`) (`KismetMathLibrary.MakeRotator` 0.0 0.0 (* AxisValue -5.0))))))

(event `InputAxisKey|MouseY`
  (params (AxisValue :type "Float (single-precision)"))
  (if (`self.IsRotating`)
    (`self.K2_SetActorRotation` (`KismetMathLibrary.ComposeRotators` (`self.K2_GetActorRotation`) (`KismetMathLibrary.MakeRotator` 0.0 (* AxisValue -5.0))))))

(event `ActivateScanPhase`
  (bind _staticmesh (`self.StaticMesh`))
  (set `PlayerController.bShowMouseCursor` false (`GameplayStatics.GetPlayerController` 0))
  (bind _cashregisterref (message `/Game/BP/BP_GameModeInterface.GetCashRegisterRef` (`GameplayStatics.GetGameMode`)))
  (`SceneComponent.K2_SetWorldLocation` (`self.StaticMesh`) (`SceneComponent.K2_GetComponentLocation` (`/Game/BP/BP_CashRegister.ItemInspect` _cashregisterref)) false false)
  (set `self.IsOnScanner` true)
  (set `self.IsRotating` true)
  (`PrimitiveComponent.SetEnableGravity` _staticmesh false)
  (`PrimitiveComponent.SetSimulatePhysics` _staticmesh false)
  (`PrimitiveComponent.SetAllPhysicsLinearVelocity` _staticmesh (0.0 0.0 0.0) true)
  (`self.EnableInput` (`GameplayStatics.GetPlayerController` 0)))

(event `DesactivateScanPhase`
  (bind _returnvalue (`GameplayStatics.GetPlayerController` 0))
  (bind _staticmesh (`self.StaticMesh`))
  (`PrimitiveComponent.SetSimulatePhysics` _staticmesh true)
  (`PrimitiveComponent.SetEnableGravity` _staticmesh true)
  (set `self.IsOnScanner` false)
  (set `self.IsRotating` false)
  (`self.DisableInput` _returnvalue)
  (set `PlayerController.bShowMouseCursor` true _returnvalue))

(fn `UserConstructionScript`)